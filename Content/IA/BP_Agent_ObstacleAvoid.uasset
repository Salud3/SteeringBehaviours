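; AI steering agent that seeks either BP_Target or a BP_Agent_Flee actor, chosen by the Target flag, while avoiding obstacles.
; Each Tick, Seek fires eight line traces at fixed world-space offsets through SetDetector, which turns hit normals into push forces.
; Any hit replaces seek steering with those forces added to the current velocity, renormalized to MaxVel.
; The result drives the Cone's physics velocity and facing, with debug arrows showing the vectors.
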(event `self.ReceiveBeginPlay`
  (set `self.CurrentVel` (0.0 0.0 100.0))
  (if (`self.Target?`)
    (bind _returnvalue (`GameplayStatics.GetActorOfClass` "/Game/IA/BP_Target.BP_Target_C"))
    (set `self.bp_Target` _returnvalue)
    (else
      (bind _returnvalue_2 (`GameplayStatics.GetActorOfClass` "/Game/IA/BP_Agent_Flee.BP_Agent_Flee_C"))
      (set `self.bp_Flee` _returnvalue_2))))

(event `self.ReceiveTick`
  (params (DeltaSeconds :type "Float (single-precision)"))
  (set `self.DTime` (+ DeltaSeconds (`self.DTime`)))
  (if (`self.Target?`)
    (`self.Seek` (`SceneComponent.K2_GetComponentLocation` (`/Game/IA/BP_Target.Sphere` (`self.bp_Target`))) false (`self.DTime`))
    (`PrimitiveComponent.SetPhysicsLinearVelocity` (`self.Cone`) (`self.CurrentVel`) false "None")
    (`self.LookAtDirection`)
    (else
      (`self.Seek` (`SceneComponent.K2_GetComponentLocation` (`/Game/IA/BP_Agent_Flee.Sphere` (`self.bp_Flee`))) true (`self.DTime`))
      (`PrimitiveComponent.SetPhysicsLinearVelocity` (`self.Cone`) (`self.CurrentVel`) false "None")
      (`self.LookAtDirection`))))

(fn `LookAtDirection`
  (`SceneComponent.K2_SetWorldRotation` (`self.Cone`) (`KismetMathLibrary.MakeRotator` (.roll (`KismetMathLibrary.FindLookAtRotation` (`SceneComponent.K2_GetComponentLocation` (`self.Cone`)) (+ (`SceneComponent.RelativeLocation` (`self.Cone`)) (`self.CurrentVel`)))) (+ (.pitch (`KismetMathLibrary.FindLookAtRotation` (`SceneComponent.K2_GetComponentLocation` (`self.Cone`)) (+ (`SceneComponent.RelativeLocation` (`self.Cone`)) (`self.CurrentVel`)))) -90.0) (.yaw (`KismetMathLibrary.FindLookAtRotation` (`SceneComponent.K2_GetComponentLocation` (`self.Cone`)) (+ (`SceneComponent.RelativeLocation` (`self.Cone`)) (`self.CurrentVel`))))) false false))

(fn `RaycastDetect`
  (params (ObstaclePos :type "Vector Structure"))
  (returns (Movement :type "Vector Structure"))
  (locals (_Movement :type "Vector Structure") (PosX :type "Float (double-precision)") (PosY :type "Float (double-precision)") (PosZ :type "Float (double-precision)")))

(fn `Seek`
  (params (TargetPos :type "Vector Structure") (Debug :type Boolean) (Timer :type "Float (double-precision)"))
  (locals (_TargetPos :type "Vector Structure") (_Debug :type Boolean) (_time :type "Float (double-precision)") (_AddPosF :type "Vector Structure") (_AddPosR :type "Vector Structure") (_AddPosL :type "Vector Structure") (`1` :type Boolean :default false) (`2` :type Boolean :default false) (`3` :type Boolean :default false) (ForceTotal :type "Vector Structure") (`4` :type Boolean) (`5` :type Boolean) (`6` :type Boolean) (`7` :type Boolean) (`8` :type Boolean) (_AddPosRR :type "Vector Structure") (_AddPosLL :type "Vector Structure") (_AddPosBF :type "Vector Structure") (_AddPosBR :type "Vector Structure") (_AddPosBL :type "Vector Structure"))
  (bind _returnvalue (`SceneComponent.K2_GetComponentLocation` (`self.Cone`)))
  (bind _returnvalue_2 (`SceneComponent.K2_GetComponentLocation` (`self.Cone`)))
  (bind _returnvalue_3 (`SceneComponent.K2_GetComponentLocation` (`self.Cone`)))
  (set `local._Debug` Debug)
  (set `local._time` Timer)
  (set `local._TargetPos` TargetPos)
  (`|ExecutionSequence`
    (:`then_0`
      (`|ExecutionSequence`
        (:`then_0`
          (bind (_posf _bool) (`self.SetDetector` (-154.0 0.0 0.0)))
          (set `local.1` _bool)
          (set `local._AddPosF` _posf))
        (:`then_1`
          (bind (_posf_2 _bool_2) (`self.SetDetector` (-154.0 90.0 0.0)))
          (set `local.2` _bool_2)
          (set `local._AddPosR` _posf_2))
        (:`then_2`
          (bind (_posf_3 _bool_3) (`self.SetDetector` (-154.0 -90.0 0.0)))
          (set `local.3` _bool_3)
          (set `local._AddPosL` _posf_3))
        (:`then_3`
          (bind (_posf_4 _bool_4) (`self.SetDetector` (0.0 -154.0 0.0)))
          (set `local.4` _bool_4)
          (set `local._AddPosRR` _posf_4))
        (:`then_4`
          (bind (_posf_5 _bool_5) (`self.SetDetector` (0.0 154.0 0.0)))
          (set `local.5` _bool_5)
          (set `local._AddPosLL` _posf_5))
        (:`then_5`
          (bind (_posf_6 _bool_6) (`self.SetDetector` (154.0 0.0 0.0)))
          (set `local.6` _bool_6)
          (set `local._AddPosBF` _posf_6))
        (:`then_6`
          (bind (_posf_7 _bool_7) (`self.SetDetector` (154.0 63.0 0.0)))
          (set `local.7` _bool_7)
          (set `local._AddPosBR` _posf_7))
        (:`then_7`
          (bind (_posf_8 _bool_8) (`self.SetDetector` (154.0 -63.0 0.0)))
          (set `local.8` _bool_8)
          (set `local._AddPosBL` _posf_8))))
    (:`then_1`
      ;[0 1 0.003194] Set Desired Vel
      (set `self.DesiredVel` (* (`KismetMathLibrary.Normal` (- (`local._TargetPos`) (`SceneComponent.K2_GetComponentLocation` (`self.Cone`)))) (`self.MaxVel`))))
    (:`then_2`
      ;[1 0.9658 0] Debug
      (`KismetSystemLibrary.DrawDebugArrow` _returnvalue_2 (+ _returnvalue_2 (`self.DesiredVel`)) 0.0 (struct :`G` 0.133177 :`B` 1.0 :`A` 1.0) 0.0 2.0))
    (:`then_3`
      ;[0 1 0.02106] SetSteering
      (set `self.SteeringForce` (* (`KismetMathLibrary.Normal` (- (`self.DesiredVel`) (`self.CurrentVel`))) (`self.MaxForce`))))
    (:`then_4`
      ;[1 0.9658 0] Debug Steering
      (if (`local._Debug`)
        (`KismetSystemLibrary.DrawDebugArrow` _returnvalue_3 (+ (+ _returnvalue_3 (`self.CurrentVel`)) (`self.SteeringForce`)) 0.0 (struct :`R` 0.036748 :`G` 1.0 :`A` 1.0) 0.0 3.0)))
    (:`then_5`
      ;[0 1 0.001744] SetCurrentFinal
      (if (or (`local.1`) (`local.2`) (`local.3`) (`local.4`) (`local.5`) (`local.6`) (`local.7`) (`local.8`))
        (set `local.ForceTotal` (+ (`local._AddPosF`) (`local._AddPosR`) (`local._AddPosL`) (`local._AddPosRR`) (`local._AddPosLL`) (`local._AddPosBF`) (`local._AddPosBR`) (`local._AddPosBL`) (`self.CurrentVel`)))
        (set `self.CurrentVel` (* (`KismetMathLibrary.Normal` (`local.ForceTotal`)) (`self.MaxVel`)))
        (else
          (set `self.CurrentVel` (* (`KismetMathLibrary.Normal` (+ (`self.CurrentVel`) (`self.SteeringForce`))) (`self.MaxVel`))))))
    (:`then_6`
      ;[1 0.9658 0] Debug Steering
      (if (`local._Debug`)
        (`KismetSystemLibrary.DrawDebugArrow` _returnvalue (+ _returnvalue (`self.CurrentVel`)) 0.0 (struct :`R` 1.0 :`B` 0.296981 :`A` 1.0) 0.0 4.0)))))

(fn `SetDetector`
  (params (VectInit :type "Vector Structure"))
  (returns (PosF :type "Vector Structure") (Bool :type Boolean))
  (locals (AddPosF :type "Vector Structure") (Bool1 :type Boolean))
  (bind _returnvalue (`SceneComponent.K2_GetComponentLocation` (`self.Cone`)))
  (set `local.AddPosF` VectInit)
  (bind (_outhit _returnvalue_2) (`KismetSystemLibrary.LineTraceSingleForObjects` :`Start` _returnvalue :`End` (+ (`local.AddPosF`) _returnvalue) :`ObjectTypes` (`self.Object Types`) :`DrawDebugType` "ForOneFrame"))
  (bind _output_get (set `local.Bool1` _returnvalue_2))
  (if _output_get
    (bind _output_get_2 (set `local.AddPosF` (* (`.Normal` (`GameplayStatics.BreakHitResult` _outhit)) (`self.MaxForce`))))
    (return _output_get_2 (`local.Bool1`))
    (else
      (set `local.AddPosF` (0.0 0.0 0.0)))))

(fn `UserConstructionScript`)