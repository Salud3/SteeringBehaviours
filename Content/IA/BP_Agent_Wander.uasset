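; AI agent that roams by steering a physics-driven Cone toward a random wander target, re-picked about every five seconds via a Delay on Tick.
; Each tick, Wander computes desired velocity and steering force, sets a constant-speed velocity on the Cone, and draws debug arrows.
; LookAtDirection pitches the Cone from its velocity.
; WanderPosition scales the current location by random factors, sometimes forcing absolute coordinates when the Cone is low.
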(event `self.ReceiveBeginPlay`
  (set `self.CurrentVel` (0.0 0.0 100.0))
  (`self.WanderPosition`))

(event `self.ReceiveTick`
  (params (DeltaSeconds :type "Float (single-precision)"))
  (`|ExecutionSequence`
    (:`then_0`
      (`KismetSystemLibrary.Delay` 5.0)
      (`self.WanderPosition`))
    (:`then_1`
      (`self.Wander` true (`self.Wander_Position`))
      (`PrimitiveComponent.SetPhysicsLinearVelocity` (`self.Cone`) (`self.CurrentVel`) false "None")
      (`self.LookAtDirection`))))

(fn `LookAtDirection`
  (`SceneComponent.K2_SetWorldRotation` (`self.Cone`) (`KismetMathLibrary.MakeRotator` (.roll (`KismetMathLibrary.FindLookAtRotation` (`SceneComponent.K2_GetComponentLocation` (`self.Cone`)) (+ (`SceneComponent.RelativeLocation` (`self.Cone`)) (`self.CurrentVel`)))) (+ (.pitch (`KismetMathLibrary.FindLookAtRotation` (`SceneComponent.K2_GetComponentLocation` (`self.Cone`)) (+ (`SceneComponent.RelativeLocation` (`self.Cone`)) (`self.CurrentVel`)))) -90.0) (.yaw (`KismetMathLibrary.FindLookAtRotation` (`SceneComponent.K2_GetComponentLocation` (`self.Cone`)) (+ (`SceneComponent.RelativeLocation` (`self.Cone`)) (`self.CurrentVel`))))) false false))

(fn `UserConstructionScript`)

(fn `Wander`
  (params (Debug :type Boolean) (DestinyPos :type "Vector Structure"))
  (locals (_DestinyPos :type "Vector Structure") (_Debug :type Boolean))
  (bind _returnvalue (`SceneComponent.K2_GetComponentLocation` (`self.Cone`)))
  (bind _returnvalue_2 (`SceneComponent.K2_GetComponentLocation` (`self.Cone`)))
  (bind _returnvalue_3 (`SceneComponent.K2_GetComponentLocation` (`self.Cone`)))
  (set `local._Debug` Debug)
  (set `local._DestinyPos` DestinyPos)
  (`|ExecutionSequence`
    (:`then_0`
      ;[0 1 0.003194] Set Desired Vel
      (set `self.DesiredVel` (* (`KismetMathLibrary.Normal` (- (`local._DestinyPos`) (`SceneComponent.K2_GetComponentLocation` (`self.Cone`)))) (`self.MaxVel`))))
    (:`then_1`
      ;[1 0.9658 0] Debug
      (if (`local._Debug`)
        (`KismetSystemLibrary.DrawDebugArrow` _returnvalue_2 (+ _returnvalue_2 (`self.DesiredVel`)) 0.0 (struct :`G` 0.133177 :`B` 1.0 :`A` 1.0) 0.0 2.0)))
    (:`then_2`
      ;[0 1 0.02106] SetSteering
      (set `self.SteeringForce` (* (`KismetMathLibrary.Normal` (- (`self.DesiredVel`) (`self.CurrentVel`))) (`self.MaxForce`))))
    (:`then_3`
      ;[1 0.9658 0] Debug Steering
      (if (`local._Debug`)
        (`KismetSystemLibrary.DrawDebugArrow` _returnvalue_3 (+ (+ _returnvalue_3 (`self.CurrentVel`)) (`self.SteeringForce`)) 0.0 (struct :`R` 0.036748 :`G` 1.0 :`A` 1.0) 0.0 3.0)))
    (:`then_4`
      ;[0 1 0.001744] SetCurrentFinal
      (set `self.CurrentVel` (* (`KismetMathLibrary.Normal` (+ (`self.CurrentVel`) (`self.SteeringForce`))) (`self.MaxVel`))))
    (:`then_5`
      ;[1 0.9658 0] Debug Steering
      (if (`local._Debug`)
        (`KismetSystemLibrary.DrawDebugArrow` _returnvalue (+ _returnvalue (`self.CurrentVel`)) 0.0 (struct :`R` 1.0 :`B` 0.296981 :`A` 1.0) 0.0 4.0)))))

(fn `WanderPosition`
  (bind _wanderradius (`self.WanderRadius`))
  (bind _returnvalue (`SceneComponent.K2_GetComponentLocation` (`self.Cone`)))
  (bind _returnvalue_2 (* (`self.WanderRadius`) -1.0))
  (bind _returnvalue_3 (- _returnvalue (* _returnvalue (`KismetMathLibrary.MakeVector` (`KismetMathLibrary.RandomFloatInRange` _returnvalue_2 _wanderradius) (`KismetMathLibrary.RandomFloatInRange` _returnvalue_2 _wanderradius) (`KismetMathLibrary.RandomFloatInRange` _returnvalue_2 _wanderradius)))))
  ;[1 1 1] SetFuturePosition
  (if (and (< (.z (`SceneComponent.K2_GetComponentLocation` (`self.Cone`))) 150.0) (or (< (.x _returnvalue_3) -1.0) (< (.y _returnvalue_3) -1.0) (< (.z _returnvalue_3) -1.0)))
    (set `self.Wander_Position` (`KismetMathLibrary.Vector_GetAbs` _returnvalue_3))
    (else
      (set `self.Wander_Position` _returnvalue_3))))