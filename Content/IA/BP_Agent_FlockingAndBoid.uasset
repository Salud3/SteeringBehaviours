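; Boid agent actor that flocks with other instances of its class by driving the physics velocity of its Cone.
; BeginPlay caches all agents and picks a random velocity.
; Each Tick sums alignment, cohesion and separation into ObjPos, treats it as a Seek destination for steering, then rotates the cone toward its velocity.
; An earlier Flock/Move version and a wander test remain unconnected.
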(event `self.ReceiveBeginPlay`
  (`self.ObtainAllForces`)
  (set `self.CurrentVel` (`KismetMathLibrary.MakeVector` (`KismetMathLibrary.RandomFloatInRange` -150.0 150.0) (`KismetMathLibrary.RandomFloatInRange` -150.0 150.0) (`KismetMathLibrary.RandomFloatInRange` -150.0 150.0))))

(event `self.ReceiveTick`
  (params (DeltaSeconds :type "Float (single-precision)"))
  (bind _cone (`self.Cone`))
  (`|ExecutionSequence`
    (:`then_0`
      (bind __vec (`self.AlingForces`)))
    (:`then_1`
      (bind __vec_2 (`self.CohesionForce`))
      (`PrimitiveComponent.SetPhysicsLinearVelocity` _cone __vec_2 false "None"))
    (:`then_2`
      (bind __vec_3 (`self.SeparationForce`))
      (`PrimitiveComponent.SetPhysicsLinearVelocity` _cone __vec_3 false "None"))
    (:`then_3`
      (bind _output_get (set `self.ObjPos` (+ __vec __vec_2 __vec_3)))
      (`self.Seek` false _output_get)
      (`PrimitiveComponent.SetPhysicsLinearVelocity` (`self.Cone`) (`self.CurrentVel`) false "None"))
    (:`then_4`
      (`self.LookAtDirection`))))

(fn `Aling`
  (returns (_Steer :type "Vector Structure"))
  (locals (Sum :type "Vector Structure") (count :type Integer) (Steer :type "Vector Structure"))
  (`|ExecutionSequence`
    (:`then_0`
      (set `local.count` 0)
      (set `local.Sum` (`KismetMathLibrary.Vector_Zero`))
      (for _array_element (`self.Actors`)
        (if (!= _array_element self)
          (set `local.Sum` (+ (`local.Sum`) (`/Game/IA/BP_Agent_FlockingAndBoid.CurrentVel` _array_element)))
          (set `local.count` (+ (`local.count`) 1)))))
    (:`then_1`
      (if (> (`local.count`) 0)
        (bind _output_get (set `local.Sum` (/ (`local.Sum`) (`local.count`))))
        (bind _output_get_2 (set `local.Sum` (* (`KismetMathLibrary.Normal` _output_get) (`self.MaxVel`))))
        (bind _output_get_3 (set `local.Steer` (- _output_get_2 (`self.CurrentVel`))))
        (set `local.Steer` (`KismetMathLibrary.ClampVectorSize` _output_get_3 0.0 (`self.MaxForce`)))
        (else
          (set `local.Sum` (`KismetMathLibrary.Vector_Zero`)))))
    (:`then_2`
      (return (`local.Steer`)))))

(fn `AlingForces`
  (returns (_vec :type "Vector Structure"))
  (locals (Vec :type "Vector Structure") (Count :type Integer))
  (`|ExecutionSequence`
    (:`then_0`
      (set `local.Vec` (`KismetMathLibrary.Vector_Zero`))
      (set `local.Count` 0)
      (for _array_element (`self.Actors`)
        (if (!= _array_element self)
          (if (> (`KismetMathLibrary.Vector_Distance` (`SceneComponent.K2_GetComponentLocation` (`self.Cone`)) (`SceneComponent.K2_GetComponentLocation` (`/Game/IA/BP_Agent_FlockingAndBoid.Cone` _array_element))) (`self.ObjDistance`))
            (set `local.Vec` (+ (`local.Vec`) (`/Game/IA/BP_Agent_FlockingAndBoid.CurrentVel` _array_element)))
            (set `local.Count` (+ (`local.Count`) 1))))))
    (:`then_1`
      (if (> (`local.Count`) 0)
        (set `local.Vec` (* (`local.Vec`) (`self.MaxForce`)))))
    (:`then_2`
      (return (`local.Vec`)))))

(fn `ApplyForce`
  (params (force :type "Vector Structure"))
  (set `self.Aceleration` (+ force (`self.Aceleration`))))

(fn `Cohere`
  (returns (_Sum :type "Vector Structure"))
  (locals (sum :type "Vector Structure") (Count :type Integer))
  (`|ExecutionSequence`
    (:`then_0`
      (set `local.Count` 0)
      (set `local.sum` (`KismetMathLibrary.Vector_Zero`))
      (for _array_element (`self.Actors`)
        (if (!= _array_element self)
          (set `local.sum` (+ (`local.sum`) (`SceneComponent.K2_GetComponentLocation` (`/Game/IA/BP_Agent_FlockingAndBoid.Cone` _array_element))))
          (set `local.Count` (+ (`local.Count`) 1)))))
    (:`then_1`
      (if (> (`local.Count`) 0)
        (set `local.sum` (/ (`local.sum`) (`local.Count`)))
        (else
          (set `local.sum` (`KismetMathLibrary.Vector_Zero`)))))
    (:`then_2`
      (return (`local.sum`)))))

(fn `CohesionForce`
  (returns (_vec :type "Vector Structure"))
  (locals (Vec :type "Vector Structure") (Count :type Integer))
  (`|ExecutionSequence`
    (:`then_0`
      (set `local.Vec` (`KismetMathLibrary.Vector_Zero`))
      (set `local.Count` 0)
      (for _array_element (`self.Actors`)
        (if (!= _array_element self)
          (set `local.Vec` (+ (`local.Vec`) (`SceneComponent.K2_GetComponentLocation` (`/Game/IA/BP_Agent_FlockingAndBoid.Cone` _array_element))))
          (set `local.Count` (+ (`local.Count`) 1)))))
    (:`then_1`
      (if (> (`local.Count`) 0)
        (bind _output_get (set `local.Vec` (/ (`local.Vec`) (`local.Count`))))
        (bind __vect (`self.Miniseek` _output_get))
        (set `local.Vec` __vect)))
    (:`then_2`
      (return (`local.Vec`)))))

(fn `Flock`
  (locals (separation :type "Vector Structure") (alignment :type "Vector Structure") (cohesion :type "Vector Structure") (Steering :type "Vector Structure"))
  (`|ExecutionSequence`
    (:`then_0`
      (bind __steer (`self.Separate`))
      (set `local.separation` __steer)
      (bind __steer_2 (`self.Aling`))
      (set `local.alignment` __steer_2)
      (bind __sum (`self.Cohere`))
      (set `local.cohesion` __sum))
    (:`then_1`
      (set `local.separation` (* (`local.separation`) 1.5))
      (bind _output_get (set `local.Steering` (+ (`local.separation`) (`local.alignment`) (`local.cohesion`))))
      (`self.ApplyForce` _output_get))))

(fn `LookAtDirection`
  (`SceneComponent.K2_SetWorldRotation` (`self.Cone`) (`KismetMathLibrary.MakeRotator` (.roll (`KismetMathLibrary.FindLookAtRotation` (`SceneComponent.K2_GetComponentLocation` (`self.Cone`)) (+ (`SceneComponent.RelativeLocation` (`self.Cone`)) (`self.CurrentVel`)))) (+ (.pitch (`KismetMathLibrary.FindLookAtRotation` (`SceneComponent.K2_GetComponentLocation` (`self.Cone`)) (+ (`SceneComponent.RelativeLocation` (`self.Cone`)) (`self.CurrentVel`)))) -90.0) (.yaw (`KismetMathLibrary.FindLookAtRotation` (`SceneComponent.K2_GetComponentLocation` (`self.Cone`)) (+ (`SceneComponent.RelativeLocation` (`self.Cone`)) (`self.CurrentVel`))))) false false))

(fn `Miniseek`
  (params (_vec :type "Vector Structure"))
  (returns (_vect :type "Vector Structure"))
  (locals (Vect :type "Vector Structure"))
  (bind _output_get (set `local.Vect` _vec))
  (bind _output_get_2 (set `local.Vect` (- _output_get (`SceneComponent.K2_GetComponentLocation` (`self.Cone`)))))
  (bind _output_get_3 (set `local.Vect` (* _output_get_2 (`self.MaxVel`))))
  (set `local.Vect` (* (`KismetMathLibrary.Normal` (- _output_get_3 (`self.CurrentVel`))) (`self.MaxForce`)))
  (return (`local.Vect`)))

(fn `Move`
  (`|ExecutionSequence`
    (:`then_0`
      (set `self.CurrentVel` (`KismetMathLibrary.Vector_Zero`)))
    (:`then_1`
      (bind _output_get (set `self.CurrentVel` (+ (`self.CurrentVel`) (`self.Aceleration`))))
      (set `self.CurrentVel` (`KismetMathLibrary.ClampVectorSize` _output_get 0.0 (`self.MaxVel`))))))

(fn `ObtainAllForces`
  (bind _outactors (`GameplayStatics.GetAllActorsOfClass` "BP_Agent_FlockingAndBoid_C"))
  (bind _output_get (set `self.Actors` _outactors))
  (for _array_element _output_get
    (if (!= _array_element self)
      (set `self.ObjPos` (+ (`self.ObjPos`) (`/Game/IA/BP_Agent_FlockingAndBoid.ObjPos` _array_element))))))

(fn `Seeek`
  (params (Target :type "Vector Structure"))
  (returns (__Steer :type "Vector Structure"))
  (locals (desired :type "Vector Structure") (steer :type "Vector Structure") (_target :type "Vector Structure"))
  (set `local._target` Target)
  (set `local.desired` (- (`local._target`) (`SceneComponent.K2_GetComponentLocation` (`self.Cone`))))
  (set `local.desired` (* (`KismetMathLibrary.Normal` (`local.desired`)) (`self.MaxVel`)))
  (bind _output_get (set `local.steer` (- (`local.desired`) (`self.CurrentVel`))))
  (bind _output_get_2 (set `local.steer` (`KismetMathLibrary.ClampVectorSize` _output_get 0.0 (`self.MaxForce`))))
  (return _output_get_2))

(fn `Seek`
  (params (Debug :type Boolean) (DestinyPos :type "Vector Structure"))
  (locals (_DestinyPos :type "Vector Structure") (_Debug :type Boolean))
  (bind _returnvalue (`SceneComponent.K2_GetComponentLocation` (`self.Cone`)))
  (bind _returnvalue_2 (`SceneComponent.K2_GetComponentLocation` (`self.Cone`)))
  (bind _returnvalue_3 (`SceneComponent.K2_GetComponentLocation` (`self.Cone`)))
  (set `local._Debug` Debug)
  (set `local._DestinyPos` DestinyPos)
  (`|ExecutionSequence`
    (:`then_0`
      ;[0 1 0.003194] Set Desired Vel
      (set `self.DesiredVel` (* (`KismetMathLibrary.Normal` (- (`self.ObjPos`) (`SceneComponent.K2_GetComponentLocation` (`self.Cone`)))) (`self.MaxVel`))))
    (:`then_1`
      ;[1 0.9658 0] Debug
      (if (`local._Debug`)
        (`KismetSystemLibrary.DrawDebugArrow` _returnvalue_2 (+ _returnvalue_2 (`self.DesiredVel`)) 0.0 (struct :`G` 0.133177 :`B` 1.0 :`A` 1.0) 0.0 2.0)))
    (:`then_2`
      ;[0 1 0.02106] SetSteering
      (set `self.SteeringForce` (* (`KismetMathLibrary.Normal` (- (`self.DesiredVel`) (`self.CurrentVel`))) (`self.MaxForce`))))
    (:`then_3`
      ;[1 0.9658 0] Debug Steering
      (if (`local._Debug`)
        (`KismetSystemLibrary.DrawDebugArrow` _returnvalue_3 (+ (+ _returnvalue_3 (`self.CurrentVel`)) (`self.SteeringForce`)) 0.0 (struct :`R` 0.036748 :`G` 1.0 :`A` 1.0) 0.0 3.0)))
    (:`then_4`
      ;[0 1 0.001744] SetCurrentFinal
      (set `self.CurrentVel` (* (`KismetMathLibrary.Normal` (+ (`self.CurrentVel`) (`self.SteeringForce`))) (`self.MaxVel`))))
    (:`then_5`
      ;[1 0.9658 0] Debug Steering
      (if (`local._Debug`)
        (`KismetSystemLibrary.DrawDebugArrow` _returnvalue (+ _returnvalue (`self.CurrentVel`)) 0.0 (struct :`R` 1.0 :`B` 0.296981 :`A` 1.0) 0.0 4.0)))))

(fn `Separate`
  (returns (_Steer :type "Vector Structure"))
  (locals (steer :type "Vector Structure") (diff :type "Vector Structure") (distance :type "Float (double-precision)") (count :type Integer))
  (`|ExecutionSequence`
    (:`then_0`
      (set `local.count` 0)
      (set `local.steer` (`KismetMathLibrary.Vector_Zero`))
      (for _array_element (`self.Actors`)
        (if (!= _array_element self)
          (bind _output_get (set `local.distance` (`KismetMathLibrary.Vector_Distance` (`SceneComponent.K2_GetComponentLocation` (`self.Cone`)) (`SceneComponent.K2_GetComponentLocation` (`/Game/IA/BP_Agent_FlockingAndBoid.Cone` _array_element)))))
          (if (< _output_get (`self.ObjDistance`))
            (bind _output_get_2 (set `local.diff` (- (`SceneComponent.K2_GetComponentLocation` (`self.Cone`)) (`SceneComponent.K2_GetComponentLocation` (`/Game/IA/BP_Agent_FlockingAndBoid.Cone` _array_element)))))
            (set `local.count` (+ (`local.count`) 1))
            (set `local.steer` (+ (`local.steer`) (/ (`KismetMathLibrary.Normal` _output_get_2) (`local.distance`))))))))
    (:`then_1`
      (if (> (`local.count`) 0)
        (set `local.steer` (/ (`local.steer`) (`local.count`)))))
    (:`then_2`
      (if (> (`KismetMathLibrary.VSize` (`local.steer`)) 0.0)
        (set `local.steer` (- (* (`KismetMathLibrary.Normal` (`local.steer`)) (`self.MaxVel`)) (`self.CurrentVel`)))))
    (:`then_3`
      (return (`local.steer`)))))

(fn `SeparationForce`
  (returns (_vec :type "Vector Structure"))
  (locals (Vec :type "Vector Structure") (Count :type Integer) (Vec_2 :type "Vector Structure") (dist :type "Float (double-precision)") (Scale :type "Float (double-precision)"))
  (`|ExecutionSequence`
    (:`then_0`
      (set `local.Vec` (`KismetMathLibrary.Vector_Zero`))
      (set `local.Count` 0)
      (for _array_element (`self.Actors`)
        (if (!= _array_element self)
          (if (< (`KismetMathLibrary.Vector_Distance` (`SceneComponent.K2_GetComponentLocation` (`self.Cone`)) (`SceneComponent.K2_GetComponentLocation` (`/Game/IA/BP_Agent_FlockingAndBoid.Cone` _array_element))) (`self.ObjDistance`))
            (bind _output_get (set `local.Vec_2` (- (`SceneComponent.K2_GetComponentLocation` (`/Game/IA/BP_Agent_FlockingAndBoid.Cone` _array_element)) (`SceneComponent.K2_GetComponentLocation` (`self.Cone`)))))
            (bind _output_get_2 (set `local.dist` (`KismetMathLibrary.FMin` (`KismetMathLibrary.VSize` _output_get) 200.0)))
            (bind _output_get_3 (set `local.Scale` (- (/ _output_get_2 200.0) 1.0)))
            (set `local.Vec_2` (* (`local.Vec_2`) _output_get_3))
            (set `local.Vec` (+ (`local.Vec`) (`local.Vec_2`)))
            (set `local.Count` (+ (`local.Count`) 1))))))
    (:`then_1`
      (if (> (`local.Count`) 0)
        (set `local.Vec` (* (`local.Vec`) (`self.MaxForce`)))))
    (:`then_2`
      (return (`local.Vec`)))))

(fn `UserConstructionScript`)