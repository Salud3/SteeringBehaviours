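; BP_Agent_Flee is a steering-behavior agent that flees from the first BP_Agent_Seek found at BeginPlay.
; Each Tick, Flee derives a desired velocity toward the seeker's Cone, then steers along current minus desired, pushing away from it.
; The result is normalized to MaxVel and applied as the Sphere's physics linear velocity, with no delta-time scaling.
; Debug arrows, always enabled from Tick, draw the flee, steering and velocity vectors.
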(event `self.ReceiveBeginPlay`
  (set `self.CurrentVel` (50.0 15.0 100.0))
  (bind _returnvalue (`GameplayStatics.GetActorOfClass` "/Game/IA/BP_Agent_Seek.BP_Agent_Seek_C"))
  (set `self.bp_Agent` _returnvalue))

(event `self.ReceiveTick`
  (params (DeltaSeconds :type "Float (single-precision)"))
  (`self.Flee` (`SceneComponent.K2_GetComponentLocation` (`/Game/IA/BP_Agent_Seek.Cone` (`self.bp_Agent`))) true)
  (`PrimitiveComponent.SetPhysicsLinearVelocity` (`self.Sphere`) (`self.CurrentVel`) false "None"))

(fn `Flee`
  (params (EnemyPos :type "Vector Structure") (Debug :type Boolean))
  (locals (_Debug :type Boolean) (_TargetPos :type "Vector Structure") (_Distance :type "Vector Structure"))
  (bind _returnvalue (`SceneComponent.K2_GetComponentLocation` (`self.Sphere`)))
  (bind _returnvalue_2 (`SceneComponent.K2_GetComponentLocation` (`self.Sphere`)))
  (bind _returnvalue_3 (`SceneComponent.K2_GetComponentLocation` (`self.Sphere`)))
  (set `local._Debug` Debug)
  (set `local._TargetPos` EnemyPos)
  (`|ExecutionSequence`
    (:`then_0`
      ;[0 1 0.003194] Set Desired Vel
      (set `self.DesiredVel` (* (`KismetMathLibrary.Normal` (`KismetMathLibrary.NegateVector` (- (`SceneComponent.K2_GetComponentLocation` (`self.Sphere`)) (`local._TargetPos`)))) (`self.MaxVel`))))
    (:`then_1`
      ;[1 0.9658 0] Debug
      (if (`local._Debug`)
        (`KismetSystemLibrary.DrawDebugArrow` _returnvalue_2 (+ _returnvalue_2 (`KismetMathLibrary.NegateVector` (`self.DesiredVel`))) 0.0 (struct :`G` 0.133177 :`B` 1.0 :`A` 1.0) 0.0 2.0)))
    (:`then_2`
      ;[0 1 0.02106] SetSteering
      (set `self.SteeringForce` (* (`KismetMathLibrary.Normal` (- (`self.CurrentVel`) (`self.DesiredVel`))) (`self.MaxForce`))))
    (:`then_3`
      ;[1 0.9658 0] Debug Steering
      (if (`local._Debug`)
        (`KismetSystemLibrary.DrawDebugArrow` _returnvalue_3 (+ (+ _returnvalue_3 (`self.CurrentVel`)) (`self.SteeringForce`)) 0.0 (struct :`R` 0.036748 :`G` 1.0 :`A` 1.0) 0.0 3.0)))
    (:`then_4`
      ;[0 1 0.001744] SetCurrentFinal
      (set `self.CurrentVel` (* (`KismetMathLibrary.Normal` (+ (`self.CurrentVel`) (`self.SteeringForce`))) (`self.MaxVel`))))
    (:`then_5`
      ;[1 0.9658 0] Debug Steering
      (if (`local._Debug`)
        (`KismetSystemLibrary.DrawDebugArrow` _returnvalue (+ _returnvalue (`self.CurrentVel`)) 0.0 (struct :`R` 1.0 :`B` 0.296981 :`A` 1.0) 0.0 4.0)))))

(fn `UserConstructionScript`)