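; BP_Seek is an actor that steers a physics-driven Cone toward ObjectivePosition using a Seek steering behavior.
; Each Tick, the offset to the target serves as desired velocity; its difference from CurrentVel is normalized, scaled by MaxForce and accumulated into CurrentVel.
; CurrentVel is then added onto the Cone's existing physics velocity, without delta-time scaling.
; A debug arrow shows the desired velocity.
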(event `self.ReceiveBeginPlay`
  (set `self.CurrentVel` (0.0 0.0 0.0)))

(event `self.ReceiveTick`
  (params (DeltaSeconds :type "Float (single-precision)"))
  (bind _returnvalue (`SceneComponent.K2_GetComponentLocation` (`self.Cone`)))
  (`|ExecutionSequence`
    (:`then_0`
      ;[1 1 1] Restaentre Objeto y Position
      (bind _output_get (set `self.DesiredVel` (- (`self.Objective_Position`) (`SceneComponent.K2_GetComponentLocation` (`self.Cone`)))))
      (`KismetSystemLibrary.DrawDebugArrow` _returnvalue (+ _returnvalue (`self.DesiredVel`)) 3.0 (struct :`G` 0.788214 :`B` 1.0 :`A` 1.0) 0.1)
      ;[1 1 1] Resta  entre Current y Desired
      (set `self.SteeringForce` (- _output_get (`self.CurrentVel`)))
      ;[1 1 1] Normalizar
      (bind _output_get_2 (set `self.SteeringForce` (`KismetMathLibrary.Normal` (`self.SteeringForce`))))
      ;[1 1 1] Steering * MaxForce
      (set `self.SteeringForce` (* _output_get_2 (`self.MaxForce`)))
      ;[1 1 1] SetCurrentFinal
      (set `self.CurrentVel` (+ (`self.CurrentVel`) (`self.SteeringForce`))))
    (:`then_1`
      (`PrimitiveComponent.SetPhysicsLinearVelocity` (`self.Cone`) (`self.CurrentVel`) true "None"))))

(fn `Suma`
  (params (A1 :type "Float (double-precision)") (A2 :type "Float (double-precision)"))
  (returns (NewParam :type "Float (double-precision)"))
  (return (+ A1 A2)))

(fn `UserConstructionScript`)