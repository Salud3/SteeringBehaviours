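; Steering-behaviour agent that arrives at either a BP_Target or a BP_Agent_Flee, chosen by the Target flag and looked up on BeginPlay.
; Each Tick, Seek steers CurrentVel toward the target at MaxVel, scaling speed down linearly with distance inside Radius.
; That velocity drives the Cone's physics, and LookAtDirection pitches the cone to face its travel.
; Debug arrows show desired, steering and current vectors.
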(event `self.ReceiveBeginPlay`
  (set `self.CurrentVel` (0.0 0.0 100.0))
  (if (`self.Target?`)
    (bind _returnvalue (`GameplayStatics.GetActorOfClass` "/Game/IA/BP_Target.BP_Target_C"))
    (set `self.bp_Target` _returnvalue)
    (else
      (bind _returnvalue_2 (`GameplayStatics.GetActorOfClass` "/Game/IA/BP_Agent_Flee.BP_Agent_Flee_C"))
      (set `self.bp_Flee` _returnvalue_2))))

(event `self.ReceiveTick`
  (params (DeltaSeconds :type "Float (single-precision)"))
  (if (`self.Target?`)
    (`self.Seek` (`SceneComponent.K2_GetComponentLocation` (`/Game/IA/BP_Target.Sphere` (`self.bp_Target`))) true)
    (`PrimitiveComponent.SetPhysicsLinearVelocity` (`self.Cone`) (`self.CurrentVel`) false "None")
    (`self.LookAtDirection`)
    (else
      (`self.Seek` (`SceneComponent.K2_GetComponentLocation` (`/Game/IA/BP_Agent_Flee.Sphere` (`self.bp_Flee`))) true)
      (`PrimitiveComponent.SetPhysicsLinearVelocity` (`self.Cone`) (`self.CurrentVel`) false "None")
      (`self.LookAtDirection`))))

(fn `LookAtDirection`
  (`SceneComponent.K2_SetWorldRotation` (`self.Cone`) (`KismetMathLibrary.MakeRotator` (.roll (`KismetMathLibrary.FindLookAtRotation` (`SceneComponent.K2_GetComponentLocation` (`self.Cone`)) (+ (`SceneComponent.RelativeLocation` (`self.Cone`)) (`self.CurrentVel`)))) (+ (.pitch (`KismetMathLibrary.FindLookAtRotation` (`SceneComponent.K2_GetComponentLocation` (`self.Cone`)) (+ (`SceneComponent.RelativeLocation` (`self.Cone`)) (`self.CurrentVel`)))) -90.0) (.yaw (`KismetMathLibrary.FindLookAtRotation` (`SceneComponent.K2_GetComponentLocation` (`self.Cone`)) (+ (`SceneComponent.RelativeLocation` (`self.Cone`)) (`self.CurrentVel`))))) false false))

(fn `Seek`
  (params (TargetPos :type "Vector Structure") (Debug :type Boolean))
  (locals (_TargetPos :type "Vector Structure") (_Debug :type Boolean))
  (bind _returnvalue (`SceneComponent.K2_GetComponentLocation` (`self.Cone`)))
  (bind _returnvalue_2 (`SceneComponent.K2_GetComponentLocation` (`self.Cone`)))
  (bind _returnvalue_3 (`SceneComponent.K2_GetComponentLocation` (`self.Cone`)))
  (bind _returnvalue_4 (- (`local._TargetPos`) (`SceneComponent.K2_GetComponentLocation` (`self.Cone`))))
  (set `local._Debug` Debug)
  (set `local._TargetPos` TargetPos)
  (`|ExecutionSequence`
    (:`then_0`
      ;[0 1 0.003194] Set Desired Vel
      (if (> (`KismetMathLibrary.VSize` _returnvalue_4) (`self.Radius`))
        (set `self.DesiredVel` (* (`KismetMathLibrary.Normal` _returnvalue_4) (`self.MaxVel`)))
        (else
          (set `self.DesiredVel` (* (`KismetMathLibrary.Normal` _returnvalue_4) (* (/ (`KismetMathLibrary.Sqrt` (+ (`KismetMathLibrary.Square` (.x _returnvalue_4)) (`KismetMathLibrary.Square` (.y _returnvalue_4)) (`KismetMathLibrary.Square` (.z _returnvalue_4)))) (`self.Radius`)) (`self.MaxVel`)))))))
    (:`then_1`
      ;[1 0.9658 0] Debug
      (if (`local._Debug`)
        (`KismetSystemLibrary.DrawDebugArrow` _returnvalue_2 (+ _returnvalue_2 (`self.DesiredVel`)) 0.0 (struct :`G` 0.133177 :`B` 1.0 :`A` 1.0) 0.0 8.0)))
    (:`then_2`
      ;[0 1 0.02106] SetSteering
      (set `self.SteeringForce` (* (`KismetMathLibrary.Normal` (- (`self.DesiredVel`) (`self.CurrentVel`))) (`self.MaxForce`))))
    (:`then_3`
      ;[1 0.9658 0] Debug Steering
      (if (`local._Debug`)
        (`KismetSystemLibrary.DrawDebugArrow` _returnvalue_3 (+ (+ _returnvalue_3 (`self.CurrentVel`)) (`self.SteeringForce`)) 0.0 (struct :`R` 0.036748 :`G` 1.0 :`A` 1.0) 0.0 3.0)))
    (:`then_4`
      ;[0 1 0.001744] SetCurrentFinal
      (if (> (`KismetMathLibrary.VSize` (- (`local._TargetPos`) (`SceneComponent.K2_GetComponentLocation` (`self.Cone`)))) (`self.Radius`))
        (set `self.CurrentVel` (* (`KismetMathLibrary.Normal` (+ (`self.CurrentVel`) (`self.SteeringForce`))) (`self.MaxVel`)))
        (else
          (set `self.CurrentVel` (`self.DesiredVel`)))))
    (:`then_5`
      ;[1 0.9658 0] Debug Steering
      (if (`local._Debug`)
        (`KismetSystemLibrary.DrawDebugArrow` _returnvalue (+ _returnvalue (`self.CurrentVel`)) 0.0 (struct :`R` 1.0 :`B` 0.296981 :`A` 1.0) 0.0 4.0)))))

(fn `Suma`
  (params (A1 :type "Float (double-precision)") (A2 :type "Float (double-precision)"))
  (returns (NewParam :type "Float (double-precision)"))
  (return (+ A1 A2)))

(fn `UserConstructionScript`)